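; BP_Helper is a collection of small vector math helpers for offsetting positions and converting normals to rotations.
; Up and down moves offset along world Z, while forward, backward, left and right moves scale the forward or right vector of a supplied rotation.
; ReverseNormal returns a rotator rather than a vector, built from the input as the X axis and offset by 180 degrees on one axis.
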(fn MoveVectorUpward
  (params (InVector :type Vector) (AddValue :type Float%20%28double-precision%29))
  (return (+ InVector (Math|Vector|MakeVector 0.0 0.0 AddValue))))

(fn MoveVectorDownward
  (params (InVector :type Vector) (SubValue :type Float%20%28double-precision%29))
  (return (- InVector (Math|Vector|MakeVector 0.0 0.0 SubValue))))

(fn MoveVectorFoward
  (params (NewParam :type Vector) (NewParam1 :type Rotator) (NewParam3 :type Float%20%28double-precision%29))
  (return (+ NewParam (* (Math|Vector|GetForwardVector NewParam1) NewParam3))))

(fn MoveVectorBackward
  (params (InVector :type Vector) (InRot :type Rotator) (sub :type Float%20%28double-precision%29))
  (return (- InVector (* (Math|Vector|GetForwardVector InRot) sub))))

(fn MoveVectorLeft
  (params (InVector :type Vector) (InRot :type Rotator) (MoveValue :type Float%20%28double-precision%29))
  (return (- InVector (* (Math|Vector|GetRightVector InRot) MoveValue))))

(fn MoveVectorRight
  (params (InVec :type Vector) (InRot :type Rotator) (MoveValue :type Float%20%28double-precision%29))
  (return (+ InVec (* (Math|Vector|GetRightVector InRot) MoveValue))))

(fn ReverseNormal
  (params (InVec :type Vector))
  (return (Math|Rotator|Delta(Rotator) (Math|Rotator|MakeRotfromX InVec) "0.000000,180.000000,0.000000")))